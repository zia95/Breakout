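; Game mode that owns the HUD and tracks lives, score and game-over state.
; On begin play it creates the BpUIHUD widget, then resets lives to the maximum and points to zero.
; Point and life events push changes straight to the HUD, with points floored at zero.
; Losing the last life sets the game-over flag and reopens the Main level after a short delay.
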(event `self.ReceiveBeginPlay`
  ;[1 1 1] create ui, set ui & display it
  (bind _returnvalue (`|CreateWidget` "/Game/Blueprints/bpUIHUD.bpUIHUD_C"))
  (bind _output_get (set `self.ui` _returnvalue))
  (`UserWidget.AddToViewport` _output_get 0)
  (`self.Reset`))

(event `Reset`
  (bind _ui (`self.ui`))
  ;[1 1 1] reset score & lives + ui
  (bind _output_get (set `self.lives` (`self.max_lives`)))
  (set `/Game/Blueprints/bpUIHUD.lives` _output_get _ui)
  (bind _output_get_2 (set `self.points` 0))
  (set `/Game/Blueprints/bpUIHUD.points` _output_get_2 _ui)
  (set `self.is_game_over` false))

(event `UpdatePoints`
  (params (points :type Integer))
  (bind _returnvalue (+ (`self.points`) points))
  ;[1 1 1] update point + ui
  (if (<= _returnvalue 0)
    (set `self.points` 0)
    (else
      (set `self.points` _returnvalue)))
  (set `/Game/Blueprints/bpUIHUD.points` (`self.points`) (`self.ui`)))

(event `LoseLife`
  (bind _lives (`self.lives`))
  ;[1 1 1] lose life + ui
  (if (<= _lives 1)
    (`self.EndGame`)
    (else
      (bind _output_get (set `self.lives` (- _lives 1)))
      (set `/Game/Blueprints/bpUIHUD.lives` _output_get (`self.ui`)))))

(event `EndGame`
  ;[1 1 1] end the game
  (set `self.is_game_over` true)
  (`KismetSystemLibrary.Delay` 3.0)
  (`GameplayStatics.OpenLevel` "Main"))

(fn `UserConstructionScript`)
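; bpBlock is a breakable block actor that awards points when hit by the ball.
; When its Block component is hit by a bpBall, it destroys itself, passes its Points to bpGameMode's UpdatePoints and plays the Collectable sound in 2D.
; The construction script creates a dynamic material instance from MatDefault and sets its color parameter to BlockColor, so each block can have its own color.
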(event `self.Block.OnComponentHit`
  (params (HitComponent :type "PrimitiveComponent Object Reference") (OtherActor :type "Actor Object Reference") (OtherComp :type "PrimitiveComponent Object Reference") (NormalImpulse :type "Vector Structure") (Hit :type "HitResult Structure (by ref)"))
  (cast `/Game/Blueprints/bpBall` OtherActor)
  (`self.K2_DestroyActor`)
  (bind _asbp_game_mode (cast `/Game/Blueprints/bpGameMode` (`GameplayStatics.GetGameMode`)))
  (`/Game/Blueprints/bpGameMode.UpdatePoints` _asbp_game_mode (`self.points`))
  (`GameplayStatics.PlaySound2D` "/Game/Audio/collectable.collectable" 1.0 1.0 0.0 null null))

(fn `UserConstructionScript`
  ;[1 1 1] set color of our block
  (bind _returnvalue (`PrimitiveComponent.CreateDynamicMaterialInstance` (`self.Block`) 0 "/Game/Materials/matDefault.matDefault" "None"))
  (`MaterialInstanceDynamic.SetVectorParameterValue` _returnvalue "color" (`self.block_color`)))
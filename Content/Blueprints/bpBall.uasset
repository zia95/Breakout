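; Ball actor for a paddle game with lives, which follows the player paddle's arrow until LaunchBall fires it with an impulse.
; Every tick it forces physics velocity to BallSpeed and snaps its heading to the nearest 45-degree diagonal by rotating, rounding yaw to 90-degree steps and unrotating.
; When destroyed, it tells the game mode to deduct a life and has the paddle spawn a new ball.
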(event `LaunchBall`
  ;[1 1 1] Launch the ball
  (set `self.is_active` true)
  (`PrimitiveComponent.AddImpulse` (`self.Ball`) (0.0 -1000.0 0.0) "None" true))

(event `self.ReceiveBeginPlay`
  ;[1 1 1] get player
  (bind _asbp_player_paddle (cast `/Game/Blueprints/bpPlayerPaddle` (`Controller.K2_GetPawn` (`GameplayStatics.GetPlayerController` 0))))
  (set `self.player_paddle` _asbp_player_paddle)
  ;[1 1 1] get game mode
  (bind _asbp_game_mode (cast `/Game/Blueprints/bpGameMode` (`GameplayStatics.GetGameMode`)))
  (set `self.game_mode` _asbp_game_mode))

(event `self.ReceiveTick`
  (params (DeltaSeconds :type "Float (single-precision)"))
  (bind _returnvalue (`KismetMathLibrary.MakeRotator` 0.0 0.0 45.0))
  (bind _ball_speed (`self.ball_speed`))
  (`self.UpdatePos`)
  ;[1 1 1] Ball angle fix
  (bind _returnvalue_2 (`PrimitiveComponent.GetPhysicsLinearVelocity` (`self.Ball`) "None"))
  (bind _returnvalue_3 (`KismetMathLibrary.ClampVectorSize` _returnvalue_2 _ball_speed _ball_speed))
  (bind (_returnvalue_roll _returnvalue_pitch _returnvalue_yaw) (`KismetMathLibrary.BreakRotator` (`KismetMathLibrary.MakeRotFromX` (`KismetMathLibrary.GreaterGreater_VectorRotator` _returnvalue_3 _returnvalue))))
  (`PrimitiveComponent.SetPhysicsLinearVelocity` (`self.Ball`) (* (`KismetMathLibrary.LessLess_VectorRotator` (`KismetMathLibrary.Conv_RotatorToVector` (`KismetMathLibrary.MakeRotator` 0.0 0.0 (`KismetMathLibrary.Conv_IntToDouble` (* (`KismetMathLibrary.Round` (/ _returnvalue_yaw 90.0)) 90)))) _returnvalue) (`KismetMathLibrary.VSize` _returnvalue_3)) false "None"))

(event `UpdatePos`
  ;[1 1 1] update position of the ball
  (if (not (`self.is_active`))
    (`self.K2_SetActorLocation` (`SceneComponent.K2_GetComponentLocation` (`/Game/Blueprints/bpPlayerPaddle.Arrow` (`self.player_paddle`))))))

(event `self.ReceiveDestroyed`
  ;[1 1 1] Spawn new ball after destroyed
  (`/Game/Blueprints/bpGameMode.LoseLife` (`self.game_mode`))
  (`/Game/Blueprints/bpPlayerPaddle.SpawnBall` (`self.player_paddle`)))

(fn `UserConstructionScript`)